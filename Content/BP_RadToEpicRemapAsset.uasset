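; Bone remap asset that translates humanoid source bone names, apparently from a Rad skeleton, into Epic mannequin bone names.
; GetRemappedBoneName switches on the incoming name and returns the matching Epic bone for root, pelvis, spine, neck, head, arms and legs.
; The mapping is a fixed one-to-one table without fingers or toes, and the switch defines no fallback for other names.
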(fn `GetRemappedBoneName`
  (params (BoneName :type Name))
  (returns (ReturnValue :type Name))
  (switch `name` BoneName
    (:`root`
      (return "root"))
    (:`Hips`
      (return "pelvis"))
    (:`Spine`
      (return "spine_01"))
    (:`Spine1`
      (return "spine_02"))
    (:`Spine2`
      (return "spine_03"))
    (:`LeftShoulder`
      (return "clavicle_l"))
    (:`LeftArm`
      (return "upperarm_l"))
    (:`LeftForeArm`
      (return "lowerarm_l"))
    (:`LeftHand`
      (return "hand_l"))
    (:`RightShoulder`
      (return "clavicle_r"))
    (:`RightArm`
      (return "upperarm_r"))
    (:`RightForeArm`
      (return "lowerarm_r"))
    (:`RightHand`
      (return "hand_r"))
    (:`Neck`
      (return "neck_01"))
    (:`Head`
      (return "head"))
    (:`LeftUpLeg`
      (return "thigh_l"))
    (:`LeftLeg`
      (return "calf_l"))
    (:`LeftFoot`
      (return "foot_l"))
    (:`RightUpLeg`
      (return "thigh_r"))
    (:`RightLeg`
      (return "calf_r"))
    (:`RightFoot`
      (return "foot_r"))))